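; BP_SecondaryLightToggle is a one-shot interactable that sends a set-active message to every light in its ConnectedLights array.
; Its box overlap, while AlreadyLit is true, registers it as the character's interact target and shows the UI prompt.
; Interact passes a DoOnce, messages the lights, clears AlreadyLit and hides the prompt, as does leaving the box.
; The construction script caches the first ThirdPersonCharacter found.
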(event OnComponentBeginOverlap(Box)
  (params (OverlappedComponent :type Primitive%20Component%20Object%20Reference) (OtherActor :type Actor%20Object%20Reference) (OtherComp :type Primitive%20Component%20Object%20Reference) (OtherBodyIndex :type Integer) (bFromSweep :type Boolean) (SweepResult :type Hit%20Result%20Structure%20%28by%20ref%29))
  (bind _character (Variables|Default|GetCharacter))
  ;[1 1 1] Activate/Deactivate interaction
  (if (== OtherActor _character)
    (if (Variables|Default|GetAlreadyLit)
      (Variables|Default|Setb_CanInteract true)
      (Variables|/Game/ThirdPersonBP/Blueprints/ThirdPersonCharacter.ThirdPersonCharacter_C|SetInteract%20E%20Object _character self)
      (Default|ToggelUion (Variables|Default|GetCharacter)))))

(event OnComponentEndOverlap(Box)
  (params (OverlappedComponent :type Primitive%20Component%20Object%20Reference) (OtherActor :type Actor%20Object%20Reference) (OtherComp :type Primitive%20Component%20Object%20Reference) (OtherBodyIndex :type Integer))
  (bind _character (Variables|Default|GetCharacter))
  ;[1 1 1] Activate/Deactivate interaction
  (if (== OtherActor _character)
    (Variables|Default|Setb_CanInteract false)
    (Variables|/Game/ThirdPersonBP/Blueprints/ThirdPersonCharacter.ThirdPersonCharacter_C|SetInteract%20E%20Object _character 0)
    (Default|ToggleUiOff (Variables|Default|GetCharacter))))

(event EventInteract
  ;[1 1 1] Toggles all lights in ConnectedLights array on/off
  (if (Variables|Default|Getb_CanInteract)
    (Utilities|FlowControl|DoOnce false
      (:Completed
        (for _array_element (Variables|Default|GetConnectedLights)
          (Class|SecondaryLightsInterface|SetLightsActive(Message) _array_element)
          (Variables|Default|SetAlreadyLit false)
          ;[1 1 1] Activate/Deactivate interaction
          (Default|ToggleUiOff (Variables|Default|GetCharacter)))))))

(fn ConstructionScript
  (bind _outactors (Actor|GetAllActorsOfClass "/Game/ThirdPersonBP/Blueprints/ThirdPersonCharacter.ThirdPersonCharacter_C"))
  (Variables|Default|SetCharacter (Utilities|Array|Get(acopy) _outactors)))