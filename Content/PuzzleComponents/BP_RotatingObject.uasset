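; BP_RotatingObject is a puzzle component that spins at a fixed yaw rate and can be toggled on and off.
; On BeginPlay, the RotateAtStart flag sets the initial RotatingMovement rate and the Rotating state.
; Despite its name, the SetLightsActive event flips that state on each call, switching the rotation rate between zero and the spin speed.
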(event EventBeginPlay
  (bind _rotatingmovement (Variables|Default|GetRotatingMovement))
  (if (Variables|Default|GetRotateAtStart)
    (Variables|/Script/Engine.RotatingMovementComponent|SetRotationRate _rotatingmovement "30.000000, 0, 0")
    (Variables|Default|SetRotating true)
    (else
      (Variables|/Script/Engine.RotatingMovementComponent|SetRotationRate _rotatingmovement "0, 0, 0")
      (Variables|Default|SetRotating false))))

(event EventSetLightsActive
  (bind _rotatingmovement (Variables|Default|GetRotatingMovement))
  (if (Variables|Default|GetRotating)
    (Variables|/Script/Engine.RotatingMovementComponent|SetRotationRate _rotatingmovement "0, 0, 0")
    (Variables|Default|SetRotating false)
    (else
      (Variables|/Script/Engine.RotatingMovementComponent|SetRotationRate _rotatingmovement "30.000000, 0, 0")
      (Variables|Default|SetRotating true))))

(fn ConstructionScript)