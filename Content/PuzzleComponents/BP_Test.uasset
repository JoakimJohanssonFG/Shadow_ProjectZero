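; Test actor in the puzzle components folder that snaps itself onto a surface in front of it when E is pressed.
; A debug-drawn visibility line trace along its forward vector supplies the new location and impact normal, without checking for a hit.
; The rotation combines a rotator built from that normal with a fixed roll and pitch offset.
; An unconnected climbing-orientation branch that builds axes from a normal never runs.
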(event EventBeginPlay)

(event Collision|EventActorBeginOverlap
  (params (OtherActor :type Actor%20Object%20Reference)))

(event EventTick
  (params (DeltaSeconds :type Float%20%28single-precision%29)))

(event Input|KeyboardEvents|E
  (params (Key :type Key%20Structure))
  (bind _returnvalue (Transformation|GetActorLocation))
  (:Pressed
    (bind _outhit (Collision|LineTraceByChannel _returnvalue (+ _returnvalue (* (Transformation|GetActorForwardVector) 5e+02)) "TraceTypeQuery1" false 0 "ForDuration"))
    (Transformation|SetActorTransform (Math|Transform|MakeTransform (.location _outhit) (Math|Rotator|CombineRotators (Math|Rotator|MakeRotfromX (.impactnormal _outhit)) (Math|Rotator|MakeRotator 9e+01 1.8e+02 0.0)) "1,1,1"))))

(fn ConstructionScript)