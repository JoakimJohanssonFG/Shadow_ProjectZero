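; BP_Container is a puzzle component that moves its static mesh along a spline when something overlaps its box.
; Box overlap plays a timeline whose track, scaled by spline length, sets the mesh's world location without sweeping.
; The timeline's Update also runs a 10-second Delay followed by Reverse, sending the mesh back along the spline.
; Any actor triggers it, as the player-character check is unconnected.
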(event OnComponentBeginOverlap(Box)
  (params (OverlappedComponent :type Primitive%20Component%20Object%20Reference) (OtherActor :type Actor%20Object%20Reference) (OtherComp :type Primitive%20Component%20Object%20Reference) (OtherBodyIndex :type Integer) (bFromSweep :type Boolean) (SweepResult :type Hit%20Result%20Structure%20%28by%20ref%29))
  (bind _newtrack_0 (Timeline|Timeline_0 Play)
    (:Update
      (Transformation|SetWorldLocation (Variables|Default|GetStaticMesh) (Spline|GetLocationatDistanceAlongSpline (Variables|Default|GetSpline) (* _newtrack_0 (Spline|GetSplineLength (Variables|Default|GetSpline))) "World") false false)
      (Utilities|FlowControl|Delay 1e+01)
      (Timeline|Timeline_0 Reverse))))

(fn ConstructionScript)