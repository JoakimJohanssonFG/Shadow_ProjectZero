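; BP_Cameraswap is a puzzle component that switches the player's view to its own camera while the ThirdPersonCharacter is inside its overlap area.
; On BeginPlay it caches the first ThirdPersonCharacter found.
; Entering registers the actor as the character's SecondaryCam, blends the view to Cam and calls SetBlobFalse on the character.
; Leaving clears SecondaryCam and blends back to the controlled pawn.
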(event EventBeginPlay
  (bind _outactors (Actor|GetAllActorsOfClass "/Game/ThirdPersonBP/Blueprints/ThirdPersonCharacter.ThirdPersonCharacter_C"))
  (Variables|Default|SetCharacter (Utilities|Array|Get(acopy) _outactors)))

(event Collision|EventActorBeginOverlap
  (params (OtherActor :type Actor%20Object%20Reference))
  (bind _character (Variables|Default|GetCharacter))
  (if (== OtherActor _character)
    (Variables|/Game/ThirdPersonBP/Blueprints/ThirdPersonCharacter.ThirdPersonCharacter_C|SetSecondaryCam _character self)
    (Game|Player|SetViewTargetwithBlend (Game|GetPlayerController 0) (Variables|Default|GetCam) 1.0 "VTBlend_Linear" 0.0 false)
    (Default|SetBlobFalse (Variables|Default|GetCharacter))))

(event EventTick
  (params (DeltaSeconds :type Float%20%28single-precision%29)))

(event Collision|EventActorEndOverlap
  (params (OtherActor :type Actor%20Object%20Reference))
  (bind _character (Variables|Default|GetCharacter))
  (if (== OtherActor _character)
    (Variables|/Game/ThirdPersonBP/Blueprints/ThirdPersonCharacter.ThirdPersonCharacter_C|SetSecondaryCam _character 0)
    (Game|Player|SetViewTargetwithBlend (Game|GetPlayerController 0) (Pawn|GetControlledPawn (Game|GetPlayerController 0)) 1.0 "VTBlend_Linear" 0.0 false)))

(fn ConstructionScript)