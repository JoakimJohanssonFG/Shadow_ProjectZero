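; Switchable puzzle spotlight that tells the ThirdPersonCharacter whether it stands in secondary light.
; SetLightsActive toggles visibility and updates the character's lit state.
; While lit, StaticMesh overlaps with the character's LightCollider enable a Tick line trace from the spotlight to check for obstacles, with DoOnce gates limiting messages to changes.
; The construction script caches the first ThirdPersonCharacter and applies the initial on/off state.
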(event OnComponentBeginOverlap(StaticMesh)
  (params (OverlappedComponent :type Primitive%20Component%20Object%20Reference) (OtherActor :type Actor%20Object%20Reference) (OtherComp :type Primitive%20Component%20Object%20Reference) (OtherBodyIndex :type Integer) (bFromSweep :type Boolean) (SweepResult :type Hit%20Result%20Structure%20%28by%20ref%29))
  ;[1 1 1] Checks if player is in lights range. If true, sets check for obstacles to true, if false to false
  (if (Variables|Default|Getb_LightOn)
    (Variables|Default|Setb_InLightZone true)
    (Development|PrintString (Utilities|GetDisplayName OtherComp))
    (if (== OtherComp (Variables|/Game/ThirdPersonBP/Blueprints/ThirdPersonCharacter.ThirdPersonCharacter_C|GetLightCollider (Variables|Default|GetCharacter)))
      (Development|PrintString "light")
      (Variables|Default|Setb_CheckObstacles true))
    (else
      (Variables|Default|Setb_InLightZone true))))

(event OnComponentEndOverlap(StaticMesh)
  (params (OverlappedComponent :type Primitive%20Component%20Object%20Reference) (OtherActor :type Actor%20Object%20Reference) (OtherComp :type Primitive%20Component%20Object%20Reference) (OtherBodyIndex :type Integer))
  ;[1 1 1] Checks if player is in lights range. If true, sets check for obstacles to true, if false to false
  (if (Variables|Default|Getb_LightOn)
    (Variables|Default|Setb_InLightZone false)
    (if (== OtherComp (Variables|/Game/ThirdPersonBP/Blueprints/ThirdPersonCharacter.ThirdPersonCharacter_C|GetLightCollider (Variables|Default|GetCharacter)))
      (Development|PrintString "light")
      (Class|CharacterInterface|SetinSecondaryLight(Message) OtherActor false)
      (Variables|Default|Setb_CheckObstacles false)
      ;[1 1 1] Checks if light hits player while in lights range. If true, sets Characters InSecondaryLight bool to true, if false to false
      (Utilities|FlowControl|DoOnce false) ; enters at Reset
    )
    (else
      (Variables|Default|Setb_InLightZone false)
      (Utilities|FlowControl|DoOnce false) ; enters at Reset
    )))

(event EventSetLightsActive
  ;[1 1 1] Toggle Light on/off
  (if (Variables|Default|Getb_LightOn)
    (Rendering|SetVisibility (Variables|Default|GetSpotLight) false false)
    (Variables|Default|Setb_CheckObstacles false)
    (Class|CharacterInterface|SetinSecondaryLight(Message) (Variables|Default|GetCharacter) false)
    (Variables|Default|Setb_LightOn false)
    (else
      (Rendering|SetVisibility (Variables|Default|GetSpotLight) true false)
      (Variables|Default|Setb_LightOn true)
      (if (Variables|Default|Getb_InLightZone)
        (Class|CharacterInterface|SetinSecondaryLight(Message) (Variables|Default|GetCharacter) true)))))

(event EventTick
  (params (DeltaSeconds :type Float%20%28single-precision%29))
  ;[1 1 1] Checks if light hits player while in lights range. If true, sets Characters InSecondaryLight bool to true, if false to false
  (if (Variables|Default|Getb_CheckObstacles)
    (bind _outhit (Collision|LineTraceByChannel (Transformation|GetWorldLocation (Variables|Default|GetSpotLight)) (Transformation|GetWorldLocation (Variables|/Game/ThirdPersonBP/Blueprints/ThirdPersonCharacter.ThirdPersonCharacter_C|GetScene (Variables|Default|GetCharacter))) "TraceTypeQuery1" false 0 "None"))
    (if (== (.hitactor _outhit) (Variables|Default|GetCharacter))
      (Utilities|FlowControl|DoOnce false :!label _label
        (:Completed
          (Class|CharacterInterface|SetinSecondaryLight(Message) (Variables|Default|GetCharacter) true)
          (goto _label_2 Reset)))
      (else
        (Utilities|FlowControl|DoOnce false :!label _label_2
          (:Completed
            (Class|CharacterInterface|SetinSecondaryLight(Message) (Variables|Default|GetCharacter) false)
            (goto _label Reset)))))))

(fn ConstructionScript
  ;[1 1 1] Set Character Ref
  (bind _outactors (Actor|GetAllActorsOfClass "/Game/ThirdPersonBP/Blueprints/ThirdPersonCharacter.ThirdPersonCharacter_C"))
  (Variables|Default|SetCharacter (Utilities|Array|Get(acopy) _outactors))
  (if (Variables|Default|Getb_LightOn)
    (Rendering|SetVisibility (Variables|Default|GetSpotLight) true false)
    (else
      (Rendering|SetVisibility (Variables|Default|GetSpotLight) false false))))